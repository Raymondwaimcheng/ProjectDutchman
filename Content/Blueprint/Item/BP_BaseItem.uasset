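; BP_BaseItem is a configurable interactable item with a mesh and proximity icons for the player character.
; Inner and outer overlap spheres swap the near and far interact icons as the player enters or leaves.
; On Interact, inspectable items spawn a BP_InspectItem far off in the world and pass it mesh, text, rotation and scale; others only print "PickUp".
; The construction script applies sphere radii, icon location, mesh, scale and debug sphere visibility.
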(event OnComponentBeginOverlap(InnerSphereCol)
  (params (OverlappedComponent :type Primitive%20Component%20Object%20Reference) (OtherActor :type Actor%20Object%20Reference) (OtherComp :type Primitive%20Component%20Object%20Reference) (OtherBodyIndex :type Integer) (bFromSweep :type Boolean) (SweepResult :type Hit%20Result%20Structure%20%28by%20ref%29))
  (if (== OtherActor (Game|GetPlayerCharacter 0))
    (Rendering|SetVisibility (Variables|Default|GetInnerInteractIcon) true false)
    (Rendering|SetVisibility (Variables|Default|GetOuterInteractIcon) false false)))

(event OnComponentEndOverlap(InnerSphereCol)
  (params (OverlappedComponent :type Primitive%20Component%20Object%20Reference) (OtherActor :type Actor%20Object%20Reference) (OtherComp :type Primitive%20Component%20Object%20Reference) (OtherBodyIndex :type Integer))
  (if (== (Game|GetPlayerCharacter 0) OtherActor)
    (Rendering|SetVisibility (Variables|Default|GetInnerInteractIcon) false false)
    (Rendering|SetVisibility (Variables|Default|GetOuterInteractIcon) true false)))

(event OnComponentBeginOverlap(OuterSphereCol)
  (params (OverlappedComponent :type Primitive%20Component%20Object%20Reference) (OtherActor :type Actor%20Object%20Reference) (OtherComp :type Primitive%20Component%20Object%20Reference) (OtherBodyIndex :type Integer) (bFromSweep :type Boolean) (SweepResult :type Hit%20Result%20Structure%20%28by%20ref%29))
  (if (== OtherActor (Game|GetPlayerCharacter 0))
    (Rendering|SetVisibility (Variables|Default|GetOuterInteractIcon) true false)))

(event OnComponentEndOverlap(OuterSphereCol)
  (params (OverlappedComponent :type Primitive%20Component%20Object%20Reference) (OtherActor :type Actor%20Object%20Reference) (OtherComp :type Primitive%20Component%20Object%20Reference) (OtherBodyIndex :type Integer))
  (if (== (Game|GetPlayerCharacter 0) OtherActor)
    (Rendering|SetVisibility (Variables|Default|GetOuterInteractIcon) false false)))

(event EventBeginPlay
  (bind _asbp_first_person_character (Utilities|Casting|CastToBP_FirstPersonCharacter (Game|GetPlayerCharacter 0)))
  (Variables|Default|SetCharacterRef _asbp_first_person_character))

(event EventInteract
  (params (Character :type BP%20First%20Person%20Character%20Object%20Reference))
  (if (Variables|Public|Interaction|Inspect|GetInspect?)
    (bind _returnvalue (Game|SpawnActorfromClass "/Game/Blueprint/Inspect/BP_InspectItem.BP_InspectItem_C" (Math|Transform|MakeTransform "10000000000.000000,0.000000,0.000000") "Undefined" "MultiplyWithRoot" 0 0))
    (Default|SetInspectRotation _returnvalue (Variables|Public|Interaction|Inspect|GetItemInspectRotation))
    (Default|SetInspectScale _returnvalue (Variables|Public|Interaction|Inspect|GetItemInspectScale))
    (Class|IFInteract|Inspect(Message) _returnvalue Character (Variables|/Script/Engine.StaticMeshComponent|GetStaticMesh (Variables|Default|GetStaticMesh)) (Variables|Mesh|GetItemName) (Variables|Mesh|GetItemDescription))
    (else
      (Development|PrintString "PickUp"))))

(fn ConstructionScript
  (bind _staticmesh (Variables|Default|GetStaticMesh))
  (Utilities|FlowControl|Sequence
    (:then_0
      ;[1 1 1] Setting for Sphere Collision
      (Components|Sphere|SetSphereRadius (Variables|Default|GetOuterSphereCol) (Variables|Public|Interaction|Setting|GetOuterSphereRadius) true)
      (Components|Sphere|SetSphereRadius (Variables|Default|GetInnerSphereCol) (Variables|Public|Interaction|Setting|GetInnerSphereRadius) true)
      ;[1 1 1] Setting Location of Icon
      (Transformation|SetRelativeLocation (Variables|Default|GetInnerInteractIcon) (Variables|Public|Interaction|Setting|GetIconLocation) false false))
    (:then_1
      ;[1 1 1] Setting Mesh
      (Components|StaticMesh|SetStaticMesh (Variables|Default|GetStaticMesh) (Variables|Mesh|GetItemMesh))
      ;[1 1 1] Setting Scale
      (Transformation|SetWorldTransform _staticmesh (Math|Transform|MakeTransform (Transformation|GetWorldLocation _staticmesh) (Transformation|GetWorldRotation _staticmesh) (Variables|Mesh|GetItemScale)) false false))
    (:then_2
      (if (Variables|Public|Interaction|Setting|GetDebugging)
        (Rendering|SetVisibility (Variables|Default|GetInnerSphereCol) true false)
        (Rendering|SetVisibility (Variables|Default|GetOuterSphereCol) true false)
        (else
          (Rendering|SetVisibility (Variables|Default|GetInnerSphereCol) false false)
          (Rendering|SetVisibility (Variables|Default|GetOuterSphereCol) false false))))))