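; Door actor with two sliding panels and a password widget for opening it.
; Interact stores the character and uses a FlipFlop to alternately show the widget with cursor and UI input, or clear all widgets and restore game-only input.
; Opening plays the right panel's timeline, whose updates trigger the left panel's timeline.
; The left timeline's updates also repeatedly run that UI cleanup.
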(event Custom|Opening
  (bind _returnvalue (Game|GetPlayerController 0))
  (Development|PrintString "Door opening")
  (bind _newtrack (Timeline|Timeline Play)
    (:Update
      (Transformation|SetRelativeLocation (Variables|Default|GetDoor_Right) _newtrack false false)
      (bind _newtrack_0 (Timeline|Timeline_0 Play)
        (:Update
          (Transformation|SetRelativeLocation (Variables|Default|GetDoor_Left) _newtrack_0 false false)
          (Viewport|RemoveAllWidgets)
          (Input|SetInputModeGameOnly _returnvalue false)
          (Variables|/Script/Engine.PlayerController|SetbShowMouseCursor _returnvalue false))))))

(event EventInteract
  (params (Character :type BP%20First%20Person%20Character%20Object%20Reference))
  (bind _returnvalue (Game|GetPlayerController 0))
  (Variables|Default|SetCharacter Character)
  (Utilities|FlowControl|FlipFlop
    (:A
      (bind _returnvalue_2 (UserInterface|CreateWidget "/Game/Blueprint/Actor/W_Password.W_Password_C"))
      (bind _output_get (Variables|Default|SetPassword%20Widget _returnvalue_2))
      (UserInterface|Viewport|AddtoViewport _output_get 0)
      (Input|SetInputModeGameandUI _returnvalue (Variables|Default|GetPassword%20Widget) "DoNotLock" true false)
      (Variables|/Script/Engine.PlayerController|SetbShowMouseCursor _returnvalue true))
    (:B
      (Viewport|RemoveAllWidgets)
      (Input|SetInputModeGameOnly _returnvalue false)
      (Variables|/Script/Engine.PlayerController|SetbShowMouseCursor _returnvalue false))))

(fn ConstructionScript)